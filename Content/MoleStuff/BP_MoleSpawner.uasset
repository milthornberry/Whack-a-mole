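; Spawner actor that places BP_Mole actors at random spawn points, starting at BeginPlay.
; SpawnMole picks a random SpawnPoints entry, spawns a mole at its transform with itself as SpawnerRef, then immediately rechecks MoleSpawned.
; This loop has no delay and repeats until MoleSpawned is true, which this graph never sets, then prints a debug string.
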(event Custom|SpawnMole
  (if (Variables|Default|GetMoleSpawned) :!label _label
    (Development|PrintString "Bool true")
    (else
      (Game|SpawnActorfromClass "/Game/MoleStuff/BP_Mole.BP_Mole_C" (Transformation|GetActorTransform (Utilities|ResolveSoftReference (.OutItem (Utilities|Array|Random (Variables|Default|GetSpawnPoints))))) "Undefined" "MultiplyWithRoot" 0 self 0)
      (goto _label))))

(event EventBeginPlay
  (CallFunction|SpawnMole))

(event Collision|EventActorBeginOverlap
  (params (OtherActor :type Actor%20Object%20Reference)))

(event EventTick
  (params (DeltaSeconds :type Float%20%28single-precision%29)))

(fn ConstructionScript)